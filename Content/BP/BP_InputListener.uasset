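; BP_InputListener listens for a Join input action and brings local players into the game, one per press.
; On BeginPlay it enables input from player controller 0, and each press runs OnJoinPressed, which switches on a ControllerId counter.
; ID 0 reuses the existing first controller, while other IDs create a new local player.
; The resulting BP_PC_Player loads its mapping context, then the counter increments.
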(event EventBeginPlay
  (Input|EnableInput (Game|GetPlayerController 0)))

(event Input|ActionEvents|InputActionJoin
  (params (Key :type Key%20Structure :default "None"))
  (:Pressed
    (CallFunction|OnJoinPressed)))

(fn ConstructionScript)

(fn OnJoinPressed
  (bind _controllerid (Variables|Default|GetControllerId))
  (switch int _controllerid
    (:Default
      (bind _returnvalue (Class|GameplayStatics|CreatePlayer _controllerid))
      (bind _asbp_pc_player (Utilities|Casting|CastToBP_PC_Player _returnvalue))
      (Default|LoadMappingContext _asbp_pc_player))
    (:0
      (bind _asbp_pc_player_2 (Utilities|Casting|CastToBP_PC_Player (Game|GetPlayerController 0)))
      (Default|LoadMappingContext _asbp_pc_player_2)))
  (Math|Integer|IncrementInt (Variables|Default|GetControllerId)))